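; BP_PlayerCharacter is the player character Blueprint that toggles a Tab menu widget.
; On BeginPlay it creates and caches WBP_TabWidget and runs its construction.
; The Tab key drives a FlipFlop that either refreshes and shows the widget with Game and UI input and mouse cursor, or removes it and restores game-only input.
; Two boolean flags track whether the menu is open.
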(event `self.ReceiveBeginPlay`
  (bind _returnvalue (`|CreateWidget` "/Game/KHJContent/UI/WBP_TabWidget.WBP_TabWidget_C"))
  (bind _output_get (set `self.TabWidgetRef` _returnvalue))
  (`/Game/KHJContent/UI/WBP_TabWidget.Construction` _output_get))

(event `Key|Tab`
  (params (Key :type "Key Structure"))
  (bind _returnvalue (`GameplayStatics.GetPlayerController` 0))
  (:`Pressed`
    (`/Engine/EditorBlueprintResources/StandardMacros.FlipFlop`
      (:`A`
        (set `self.TabBool` true)
        (set `self.TabOn` true)
        (`TabWidget.SetTabWidget` (stale `self.ReceiveBeginPlay` _output_get))
        (`WidgetBlueprintLibrary.SetInputMode_GameAndUIEx` _returnvalue (stale `self.ReceiveBeginPlay` _output_get))
        (set `PlayerController.bShowMouseCursor` true _returnvalue)
        (`UserWidget.AddToViewport` (stale `self.ReceiveBeginPlay` _output_get) 0))
      (:`B`
        (set `self.TabBool` false)
        (set `self.TabOn` false)
        (`WidgetBlueprintLibrary.SetInputMode_GameOnly` _returnvalue)
        (set `PlayerController.bShowMouseCursor` false _returnvalue)
        (`Widget.RemoveFromParent` (stale `self.ReceiveBeginPlay` _output_get))))))

(fn `UserConstructionScript`)