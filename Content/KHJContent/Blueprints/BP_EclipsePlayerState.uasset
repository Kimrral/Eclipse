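; Player state for the Eclipse game that relays inventory actions for player characters and keeps a cached copy of the inventory.
; Add, remove and cache requests pass through server-to-multicast event chains into the character's tab widget, with caching done only on authority.
; Removal decrements or clears the dragged slot and spawns the item's actor at the player's location.
; The cached array feeds the widget's dead-body search.
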(event `self.InventoryCaching`
  (params (PlayerCharacterRef :type "PlayerCharacter Object Reference"))
  ;[1 1 1] Inventory Caching RPC
  (`self.Inventory Caching Server` PlayerCharacterRef))

(event `Inventory Caching Multicast`
  (params (`Player Character Ref` :type "PlayerCharacter Object Reference"))
  ;[1 1 1] Inventory Caching RPC
  (`/Engine/EditorBlueprintResources/ActorMacros.Switch Has Authority`
    (:`Authority`
      (bind _asbp_player_character (cast `/Game/KHJContent/Blueprints/BP_PlayerCharacter` `Player Character Ref`))
      (bind _tabwidgetref (`/Game/KHJContent/Blueprints/BP_PlayerCharacter.TabWidgetRef` _asbp_player_character))
      (bind _inventorystructarray (`/Game/KHJContent/UI/WBP_TabWidget.InventoryStructArray` _tabwidgetref))
      (`KismetArrayLibrary.Array_Clear` _inventorystructarray)
      (for (_array_element _array_index) (`/Game/KHJContent/UI/WBP_TabWidget.WBPInventoryArray` _tabwidgetref)
        (`KismetArrayLibrary.Array_Add` _inventorystructarray (`/Game/KHJContent/UI/WBP_Inventory.InventoryStruct` _array_element))
        (if (== _array_index 29)
          (break)))
      (set `self.CachedInventoryStructArray` _inventorystructarray))))

(event `Inventory Caching Server`
  (params (`Player Character Ref` :type "PlayerCharacter Object Reference"))
  ;[1 1 1] Inventory Caching RPC
  (`self.Inventory Caching Multicast` `Player Character Ref`))

(event `Inventory Caching WidgetCall`
  (params (`Player Character Ref` :type "PlayerCharacter Object Reference"))
  ;[1 1 1] Inventory Caching RPC
  (`self.Inventory Caching Server` `Player Character Ref`))

(event `AddToInventoryServer`
  (params (`Player Character Ref` :type "PlayerCharacter Object Reference") (InventoryStructRef :type "/Game/KHJContent/UI/S_Inventory Structure (by ref)"))
  ;[1 1 1] Add To Inventory RPC
  (`self.AddToInventoryMulticast` `Player Character Ref` InventoryStructRef))

(event `AddToInventoryMulticast`
  (params (`Player Character Ref` :type "PlayerCharacter Object Reference") (InventoryStructRef :type "/Game/KHJContent/UI/S_Inventory Structure"))
  ;[1 1 1] Add To Inventory RPC
  (bind _asbp_player_character (cast `/Game/KHJContent/Blueprints/BP_PlayerCharacter` `Player Character Ref`))
  (`/Engine/EditorBlueprintResources/StandardMacros.IsValid` _asbp_player_character
    (:`Is Valid`
      (`/Game/KHJContent/UI/WBP_TabWidget.AddToInventory` (`/Game/KHJContent/Blueprints/BP_PlayerCharacter.TabWidgetRef` _asbp_player_character) InventoryStructRef))))

(event `AddToInventory`
  (params (PlayerCharacterRef :type "PlayerCharacter Object Reference") (InventoryStructRef :type "/Game/KHJContent/UI/S_Inventory Structure (by ref)"))
  ;[1 1 1] Add To Inventory RPC
  (`self.AddToInventoryServer` PlayerCharacterRef InventoryStructRef))

(event `RemoveFromInventoryServer`
  (params (`Player Character Ref` :type "PlayerCharacter Object Reference"))
  ;[1 1 1] Remove From Inventory RPC
  (`self.RemoveFromInventoryMulticast` `Player Character Ref`))

(event `RemoveFromInventoryMulticast`
  (params (`Player Character Ref` :type "PlayerCharacter Object Reference"))
  ;[1 1 1] Remove From Inventory RPC
  (`KismetSystemLibrary.PrintString` "Hello")
  (bind _asbp_player_character (cast `/Game/KHJContent/Blueprints/BP_PlayerCharacter` `Player Character Ref`))
  (`/Engine/EditorBlueprintResources/StandardMacros.IsValid` _asbp_player_character
    (:`Is Valid`
      (bind _dragcountcache (`/Game/KHJContent/UI/WBP_TabWidget.DragCountCache` (`/Game/KHJContent/Blueprints/BP_PlayerCharacter.TabWidgetRef` _asbp_player_character)))
      (if (> _dragcountcache 1)
        (set `/Game/KHJContent/UI/WBP_Inventory.Count` (- _dragcountcache 1) (stale `RemoveFromInventory` InventoryObjectRef))
        (`/Game/KHJContent/UI/WBP_Inventory.InventoryUpdate` (stale `RemoveFromInventory` InventoryObjectRef) (stale `RemoveFromInventory` DragCachedStruct))
        (bind (_name _icon _thumbnail _showname _itemdescription _itemtype _typecolor _actorreference) (break `/Game/KHJContent/UI/S_Inventory` (stale `RemoveFromInventory` DragCachedStruct)))
        (bind _returnvalue (`KismetMathLibrary.Conv_VectorToTransform` (`self.K2_GetActorLocation` (stale `RemoveFromInventory` PlayerCharacterRef))))
        (`|SpawnActorFromClass` _actorreference _returnvalue "Undefined" "OverrideRootScale" null null)
        (set `/Game/KHJContent/UI/WBP_Inventory.IsFilled` true (stale `RemoveFromInventory` InventoryObjectRef))
        (else
          (`/Game/KHJContent/UI/WBP_Inventory.SetInventoryNull` (stale `RemoveFromInventory` InventoryObjectRef))
          (`|SpawnActorFromClass` _actorreference _returnvalue "Undefined" "OverrideRootScale" null null))))))

(event `RemoveFromInventory`
  (params (PlayerCharacterRef :type "PlayerCharacter Object Reference") (InventoryObjectRef :type "/Game/KHJContent/UI/WBP_Inventory Object Reference") (DragCachedStruct :type "/Game/KHJContent/UI/S_Inventory Structure"))
  ;[1 1 1] Remove From Inventory RPC
  (`self.RemoveFromInventoryServer` PlayerCharacterRef))

(event `self.DeadBodyWidgetSettings`
  (params (DeadPlayerCharacterRef :type "PlayerCharacter Object Reference") (DeadPlayerState :type "EclipsePlayerState Object Reference"))
  (bind _cachedinventorystructarray (`self.CachedInventoryStructArray`))
  ;[1 1 1] Dead Body Widget Settings RPC
  (bind _asbp_player_character (cast `/Game/KHJContent/Blueprints/BP_PlayerCharacter` DeadPlayerCharacterRef))
  (`/Engine/EditorBlueprintResources/StandardMacros.IsValid` _asbp_player_character
    (:`Is Valid`
      (for _ _cachedinventorystructarray
        _)
      (`/Game/KHJContent/UI/WBP_TabWidget.SearchDeadBodyInventory` (`/Game/KHJContent/Blueprints/BP_PlayerCharacter.TabWidgetRef` _asbp_player_character) _cachedinventorystructarray))))

(fn `UserConstructionScript`)